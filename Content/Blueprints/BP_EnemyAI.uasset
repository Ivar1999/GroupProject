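; Enemy AI pawn that chases the player on sight and drains sanity on contact.
; When PawnSensing sees a pawn, it waits a short delay, then runs AIMoveTo toward it if it is BP_PlayerCharacter.
; A hit on the PickupRange component by the player subtracts a fixed amount from CurrentSanity.
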(event `self.PawnSensing.OnSeePawn`
  (params (Pawn :type "Pawn Object Reference"))
  (`KismetSystemLibrary.Delay` 0.7)
  (bind _asbp_player_character (cast `/Game/Blueprints/BP_PlayerCharacter` Pawn))
  (`|AIMoveTo` self (0.0 0.0 0.0) _asbp_player_character))

(event `self.PickupRange.OnComponentHit`
  (params (HitComponent :type "PrimitiveComponent Object Reference") (OtherActor :type "Actor Object Reference") (OtherComp :type "PrimitiveComponent Object Reference") (NormalImpulse :type "Vector Structure") (Hit :type "HitResult Structure (by ref)"))
  (cast `/Game/Blueprints/BP_PlayerCharacter` OtherActor)
  (set `self.CurrentSanity` (- (`self.CurrentSanity`) 25)))

(fn `UserConstructionScript`
  (`parent.UserConstructionScript`))